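; BP_WindZone is a spherical wind area that pushes physics-simulating helicopters (BP_Heli_Master) along its arrow's direction.
; Sphere overlaps add and remove helicopter root meshes from an array, and the construction script sizes the sphere from WindAreaSize.
; A looping timer, running only while needed, applies mass-independent force scaled by WindStrength and reports wind shear, yaw and speed to each helicopter.
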(event `self.Sphere.OnComponentBeginOverlap`
  (params (OverlappedComponent :type "PrimitiveComponent Object Reference") (OtherActor :type "Actor Object Reference") (OtherComp :type "PrimitiveComponent Object Reference") (OtherBodyIndex :type Integer) (bFromSweep :type Boolean) (SweepResult :type "HitResult Structure (by ref)"))
  (bind _rootcomponent (`Actor.RootComponent` OtherActor))
  ;[1 1 1] Overlap Events
  ;[1 1 1] Add the helicopter to the array of under wind influence actors
  (cast `/Game/PBHeli/HelicopterBp/Blueprints/BP_Heli_Master` OtherActor)
  (bind _asstatic_mesh_component (cast `StaticMeshComponent` _rootcomponent))
  (if (`SceneComponent.IsSimulatingPhysics` _rootcomponent "None")
    (`KismetArrayLibrary.Array_AddUnique` (`self.ArrayOfMeshComponents`) _asstatic_mesh_component)
    ;[1 1 1] If the timer is not existing create a timer to apply wind force
    (if (not (`KismetSystemLibrary.K2_TimerExistsHandle` (`self.WindHandle`)))
      (bind _returnvalue (`KismetSystemLibrary.K2_SetTimerDelegate` (delegate `WindAffectedTick`) 0.02 true))
      (set `self.WindHandle` _returnvalue))))

(event `WindAffectedTick`
  (bind (_returnvalue_roll _returnvalue_pitch _returnvalue_yaw) (`KismetMathLibrary.BreakRotator` (`self.K2_GetActorRotation`)))
  ;[1 1 1] Apply Wind Force
  (if (> (`KismetArrayLibrary.Array_Length` (`self.ArrayOfMeshComponents`)) 0)
    (for (_array_element _array_index) (`self.ArrayOfMeshComponents`)
      (`/Engine/EditorBlueprintResources/StandardMacros.IsValid` _array_element
        (:`Is Valid`
          (`PrimitiveComponent.AddForce` _array_element (* (`SceneComponent.GetForwardVector` (`self.Arrow`)) (`self.WindStrength`)) "None" true)
          (bind _asbp_heli_master (cast `/Game/PBHeli/HelicopterBp/Blueprints/BP_Heli_Master` (`ActorComponent.GetOwner` _array_element)))
          (`/Game/PBHeli/HelicopterBp/Blueprints/BP_Heli_Master.EventWindShear` _asbp_heli_master true _returnvalue_yaw (`self.WindStrength`)))
        (:`Is Not Valid`
          (`KismetArrayLibrary.Array_Remove` (`self.ArrayOfMeshComponents`) _array_index))))
    (else
      ;[1 1 1] Close Timer
      (`KismetSystemLibrary.K2_ClearAndInvalidateTimerHandle` (`self.WindHandle`)))))

(event `self.Sphere.OnComponentEndOverlap`
  (params (OverlappedComponent :type "PrimitiveComponent Object Reference") (OtherActor :type "Actor Object Reference") (OtherComp :type "PrimitiveComponent Object Reference") (OtherBodyIndex :type Integer))
  ;[1 1 1] Overlap Events
  ;[1 1 1] Remove The Helicopter from the array of under wind influence actors
  (bind _asstatic_mesh_component (cast `StaticMeshComponent` (`Actor.RootComponent` OtherActor)))
  (if (`SceneComponent.IsSimulatingPhysics` _asstatic_mesh_component "None")
    (`KismetArrayLibrary.Array_RemoveItem` (`self.ArrayOfMeshComponents`) _asstatic_mesh_component)))

(fn `UserConstructionScript`
  ;[1 1 1] Simply adjust sphere radius for the overlap event
  (`SphereComponent.SetSphereRadius` (`self.Sphere`) (`self.WindAreaSize`) true))