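; Static helicopter prop Blueprint whose paint, camo and roughness are customized through its variables at construction time.
; The construction script clears cached arrays, then matches each mesh material slot to known materials, creating dynamic instances grouped as exterior, interior, tyres and lights.
; It then applies roughness, camo and optional color to exteriors and interiors, and roughness only to tyres; light instances are created but left unmodified.
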(fn `F_ClearMatInstance`
  (bind _arrayofdynmats_tyres (`self.ArrayOfDynMats_TYRES`))
  (bind _arrayofdynmats_lights (`self.ArrayOfDynMats_Lights`))
  (bind _arrayofdynmats_interiors (`self.ArrayOfDynMats_INTERIORS`))
  (bind _arrayofdynmats_exteriors (`self.ArrayOfDynMats_EXTERIORS`))
  (`KismetArrayLibrary.Array_Clear` _arrayofdynmats_exteriors)
  (`KismetArrayLibrary.Array_Resize` _arrayofdynmats_exteriors)
  (`KismetArrayLibrary.Array_Clear` _arrayofdynmats_interiors)
  (`KismetArrayLibrary.Array_Resize` _arrayofdynmats_interiors)
  (`KismetArrayLibrary.Array_Clear` _arrayofdynmats_tyres)
  (`KismetArrayLibrary.Array_Resize` _arrayofdynmats_tyres)
  (`KismetArrayLibrary.Array_Clear` _arrayofdynmats_lights)
  (`KismetArrayLibrary.Array_Resize` _arrayofdynmats_lights))

(fn `F_GetMatinstance`
  (locals (CurrentLoopId :type Integer) (CurrentLoopMat :type "MaterialInterface Object Reference"))
  (bind _currentloopmat (`local.CurrentLoopMat`))
  (for (_array_element _array_index) (`MeshComponent.GetMaterials` (`self.SM_Heli_Full`))
    (set `local.CurrentLoopId` _array_index)
    (set `local.CurrentLoopMat` _array_element)
    (if (== (`local.CurrentLoopMat`) "/Game/PBHeli/HelicopterBp/Materials/MI_BH_Exterior.MI_BH_Exterior")
      (bind _returnvalue (`PrimitiveComponent.CreateDynamicMaterialInstance` (`self.SM_Heli_Full`) (`local.CurrentLoopId`) (`local.CurrentLoopMat`) "None"))
      (`KismetArrayLibrary.Array_Add` (`self.ArrayOfDynMats_EXTERIORS`) _returnvalue)
      (elif (or (== _currentloopmat "/Game/PBHeli/HelicopterBp/Materials/MI_BH_Interior_a_Inst.MI_BH_Interior_a_Inst") (== _currentloopmat "/Game/PBHeli/HelicopterBp/Materials/MI_BH_Interior_b_Inst.MI_BH_Interior_b_Inst") (== _currentloopmat "/Game/PBHeli/HelicopterBp/Materials/MI_BH_Interior_c_Inst.MI_BH_Interior_c_Inst"))
        (bind _returnvalue_2 (`PrimitiveComponent.CreateDynamicMaterialInstance` (`self.SM_Heli_Full`) (`local.CurrentLoopId`) (`local.CurrentLoopMat`) "None"))
        (`KismetArrayLibrary.Array_Add` (`self.ArrayOfDynMats_INTERIORS`) _returnvalue_2)
        (elif (== (`local.CurrentLoopMat`) "/Game/PBHeli/HelicopterBp/Materials/MI_BH_Tire_Inst.MI_BH_Tire_Inst")
          (bind _returnvalue_3 (`PrimitiveComponent.CreateDynamicMaterialInstance` (`self.SM_Heli_Full`) (`local.CurrentLoopId`) (`local.CurrentLoopMat`) "None"))
          (`KismetArrayLibrary.Array_Add` (`self.ArrayOfDynMats_TYRES`) _returnvalue_3)
          (elif (or (== (`local.CurrentLoopMat`) "/Game/PBHeli/HelicopterBp/Materials/M_EmissiveColor.M_EmissiveColor") (== (`local.CurrentLoopMat`) "/Game/PBHeli/HelipadBP/Materials/MI_EmissiveColor_InstGreen.MI_EmissiveColor_InstGreen") (== (`local.CurrentLoopMat`) "/Game/PBHeli/HelipadBP/Materials/MI_EmissiveColor_InstRed.MI_EmissiveColor_InstRed") (== (`local.CurrentLoopMat`) "/Game/PBHeli/HelipadBP/Materials/MI_EmissiveColor_InstStrobeRed.MI_EmissiveColor_InstStrobeRed") (== (`local.CurrentLoopMat`) "/Game/PBHeli/HelipadBP/Materials/MI_EmissiveColor_InstStrobeWhite.MI_EmissiveColor_InstStrobeWhite") (== (`local.CurrentLoopMat`) "/Game/PBHeli/HelipadBP/Materials/MI_EmissiveColor_InstWhiteStrong.MI_EmissiveColor_InstWhiteStrong"))
            (bind _returnvalue_4 (`PrimitiveComponent.CreateDynamicMaterialInstance` (`self.SM_Heli_Full`) (`local.CurrentLoopId`) (`local.CurrentLoopMat`) "None"))
            (`KismetArrayLibrary.Array_Add` (`self.ArrayOfDynMats_Lights`) _returnvalue_4)))))))

(fn `F_SetMaterials`
  ;[1 0.9903 0.07997] Customize Color for interiors and exteriors
  (for _array_element (`self.ArrayOfDynMats_EXTERIORS`)
    (`MaterialInstanceDynamic.SetScalarParameterValue` _array_element "Roughness" (`self.EXT_RoughnessValue`))
    (`MaterialInstanceDynamic.SetScalarParameterValue` _array_element "Camo?" (`KismetMathLibrary.SelectFloat` 1.0 0.0 (`self.UseCamo?`)))
    (`MaterialInstanceDynamic.SetScalarParameterValue` _array_element "Color?" (`KismetMathLibrary.SelectFloat` 1.0 0.0 (`self.AddColor?`)))
    (if (`self.AddColor?`)
      (`MaterialInstanceDynamic.SetVectorParameterValue` _array_element "Color" (`self.ExtColor`))))
  (for _array_element_2 (`self.ArrayOfDynMats_INTERIORS`)
    (`MaterialInstanceDynamic.SetScalarParameterValue` _array_element_2 "Roughness" (`self.INT_RoughnessValue_0`))
    (`MaterialInstanceDynamic.SetScalarParameterValue` _array_element_2 "Camo?" (`KismetMathLibrary.SelectFloat` 1.0 0.0 (`self.UseCamo?`)))
    (`MaterialInstanceDynamic.SetScalarParameterValue` _array_element_2 "Color?" (`KismetMathLibrary.SelectFloat` 1.0 0.0 (`self.AddColor?`)))
    (if (`self.AddColor?`)
      (`MaterialInstanceDynamic.SetVectorParameterValue` _array_element_2 "Color" (`self.IntColor`))))
  (for _array_element_3 (`self.ArrayOfDynMats_TYRES`)
    (`MaterialInstanceDynamic.SetScalarParameterValue` _array_element_3 "Roughness" (`self.Tires_RoughnessValue_1`))))

(fn `UserConstructionScript`
  (`self.F_ClearMatInstance`)
  (`self.F_GetMatinstance`)
  (`self.F_SetMaterials`))